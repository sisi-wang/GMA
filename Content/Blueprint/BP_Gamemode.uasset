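; Game mode that directs BP_KING's movement: a looping walk along splines and event-driven diversions.
; After BeginPlay, chained timelines move the king along three splines from BP_Spline_king1, pausing between each.
; Bookbasket lerps him to a fixed point, fire_bookbasket to BP_Escape, and Jewellery sends him once to BP_POINT via AI MoveTo.
; These diversions call stop events to interrupt the walk or one another.
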(event Custom|Bookbasket
  (bind _returnvalue (Actor|GetActorOfClass "/Game/Blueprint/BP_KING.BP_KING_C"))
  (Variables|Default|Setbp_king _returnvalue)
  (bind _output_get (Variables|Default|SetP_location (Transformation|GetActorLocation (Variables|Default|Getbp_king))))
  (Utilities|FlowControl|Sequence
    (:then_0
      (bind _新建轨道_0 (Timeline|时间轴_0 Play)
        (:Update
          (Transformation|SetActorTransform (Variables|Default|Getbp_king) (Math|Transform|MakeTransform (Math|Vector|Lerp(Vector) _output_get "7221.000000,-3815.000000,4005.000000" _新建轨道_0) "0, 0, 0" "1.000000,1.000000,1.000000")))))
    (:then_1
      (CallFunction|STOPJEWELLERY))
    (:then_2
      (CallFunction|StopKingWalk))))

(event Custom|fire_bookbasket
  (bind _returnvalue (Actor|GetActorOfClass "/Game/Blueprint/BP_KING.BP_KING_C"))
  (bind _output_get (Variables|Default|Setbp_king _returnvalue))
  (bind _returnvalue_2 (Actor|GetActorOfClass "/Game/Blueprint/BP_Escape.BP_Escape_C"))
  (Utilities|FlowControl|Sequence
    (:then_0
      (CallFunction|StopKingWalk))
    (:then_1
      (bind _新建轨道_0 (Timeline|时间轴_1 Play)
        (:Update
          (Transformation|SetActorTransform (Variables|Default|Getbp_king) (Math|Transform|MakeTransform (Math|Vector|Lerp(Vector) (Transformation|GetActorLocation _output_get) (Transformation|GetActorLocation _returnvalue_2) _新建轨道_0) "0, 0, 0" "1.000000,1.000000,1.000000")))))
    (:then_2
      (CallFunction|STOPJEWELLERY))
    (:then_3
      (CallFunction|STOPBOOKBASKET))))

(event Custom|Jewellery
  (Utilities|FlowControl|DoOnce false
    (:Completed
      (bind _returnvalue (Actor|GetActorOfClass "/Game/Blueprint/BP_KING.BP_KING_C"))
      (bind _output_get (Variables|Default|Setbp_king _returnvalue))
      (Utilities|FlowControl|Sequence
        (:then_0
          (CallFunction|StopKingWalk))
        (:then_1
          (bind _returnvalue_2 (Actor|GetActorOfClass "/Game/Blueprint/BP_POINT.BP_POINT_C"))
          (Utilities|FlowControl|Delay 1.0)
          (AI|AIMoveTo (Variables|Default|Getbp_king) (Transformation|GetWorldLocation (Variables|/Game/Blueprint/BP_POINT.BP_POINT_C|GetSphere _returnvalue_2)) 0 5.0 false))
        (:then_2
          (CallFunction|STOPBOOKBASKET))))))

(event Custom|stop_king%20walk
  (bind _bp_spline_king (Variables|Default|Getbp_spline_king))
  (bind _spline2 (Variables|/Game/Blueprint/BP_Spline_king1.BP_Spline_king1_C|GetSpline2 _bp_spline_king))
  (Utilities|FlowControl|Sequence
    (:then_0
      (bind _新建轨道_0 (Timeline|时间轴 Stop)
        (:Update
          (Transformation|SetActorTransform (Variables|Default|Getbp_king) (Math|Transform|MakeTransform (.location (Spline|GetTransformatDistanceAlongSpline (Variables|/Game/Blueprint/BP_Spline_king1.BP_Spline_king1_C|GetSpline (stale EventBeginPlay _returnvalue)) (Math|Float|Lerp 0.0 (Spline|GetSplineLength (Variables|/Game/Blueprint/BP_Spline_king1.BP_Spline_king1_C|GetSpline (stale EventBeginPlay _returnvalue))) _新建轨道_0) "World" false)) (.rotation (Spline|GetTransformatDistanceAlongSpline (Variables|/Game/Blueprint/BP_Spline_king1.BP_Spline_king1_C|GetSpline (stale EventBeginPlay _returnvalue)) (Math|Float|Lerp 0.0 (Spline|GetSplineLength (Variables|/Game/Blueprint/BP_Spline_king1.BP_Spline_king1_C|GetSpline (stale EventBeginPlay _returnvalue))) _新建轨道_0) "World" false)) "1.000000,1.000000,1.000000")))
        (:Finished
          (Utilities|FlowControl|Delay 4.0)
          (bind _新建轨道_0_2 (Timeline|时间轴_2 PlayFromStart)
            (:Update
              (Transformation|SetActorTransform (Variables|Default|Getbp_king) (Math|Transform|MakeTransform (.location (Spline|GetTransformatDistanceAlongSpline (Variables|/Game/Blueprint/BP_Spline_king1.BP_Spline_king1_C|GetSpline1 (stale EventBeginPlay _returnvalue)) (Math|Float|Lerp 0.0 (Spline|GetSplineLength (Variables|/Game/Blueprint/BP_Spline_king1.BP_Spline_king1_C|GetSpline1 (stale EventBeginPlay _returnvalue))) _新建轨道_0_2) "World" false)) (.rotation (Spline|GetTransformatDistanceAlongSpline (Variables|/Game/Blueprint/BP_Spline_king1.BP_Spline_king1_C|GetSpline1 (stale EventBeginPlay _returnvalue)) (Math|Float|Lerp 0.0 (Spline|GetSplineLength (Variables|/Game/Blueprint/BP_Spline_king1.BP_Spline_king1_C|GetSpline1 (stale EventBeginPlay _returnvalue))) _新建轨道_0_2) "World" false)) "1.000000,1.000000,1.000000")))
            (:Finished
              (Utilities|FlowControl|Delay 3.0)
              (bind _新建轨道_0_3 (Timeline|时间轴_5 Play)
                (:Update
                  (Transformation|SetActorTransform (Variables|Default|Getbp_king) (Math|Transform|MakeTransform (.location (Spline|GetTransformatDistanceAlongSpline _spline2 (Math|Float|Lerp 0.0 (Spline|GetSplineLength _spline2) _新建轨道_0_3) "World" false)) (.rotation (Spline|GetTransformatDistanceAlongSpline _spline2 (Math|Float|Lerp 0.0 (Spline|GetSplineLength _spline2) _新建轨道_0_3) "World" false)) "1.000000,1.000000,1.000000")))
                (:Finished
                  (Utilities|FlowControl|Delay 5.0)
                  (CallFunction|Looping))))))))
    (:then_2
      (Timeline|时间轴_2 Stop))))

(event Custom|STOP_BOOKBASKET
  (bind _新建轨道_0 (Timeline|时间轴_0 Stop)
    (:Update
      (Transformation|SetActorTransform (Variables|Default|Getbp_king) (Math|Transform|MakeTransform (Math|Vector|Lerp(Vector) (stale Custom|Bookbasket _output_get) "7221.000000,-3815.000000,4005.000000" _新建轨道_0) "0, 0, 0" "1.000000,1.000000,1.000000")))))

(event Custom|STOP_JEWELLERY
  (bind _新建轨道_0 (Timeline|时间轴_3 Stop)
    (:Update
      (Transformation|SetActorTransform (Variables|Default|Getbp_king) (Math|Transform|MakeTransform (Math|Vector|Lerp(Vector) (Transformation|GetActorLocation (stale Custom|Jewellery _output_get)) "7221.000000,-3815.000000,4005.000000" _新建轨道_0) "0, 0, 0" "1.000000,1.000000,1.000000")))))

(event Custom|looping
  (bind _bp_spline_king (Variables|Default|Getbp_spline_king))
  (bind _spline2 (Variables|/Game/Blueprint/BP_Spline_king1.BP_Spline_king1_C|GetSpline2 _bp_spline_king))
  (bind _新建轨道_0 (Timeline|时间轴 PlayFromStart)
    (:Update
      (Transformation|SetActorTransform (Variables|Default|Getbp_king) (Math|Transform|MakeTransform (.location (Spline|GetTransformatDistanceAlongSpline (Variables|/Game/Blueprint/BP_Spline_king1.BP_Spline_king1_C|GetSpline (stale EventBeginPlay _returnvalue)) (Math|Float|Lerp 0.0 (Spline|GetSplineLength (Variables|/Game/Blueprint/BP_Spline_king1.BP_Spline_king1_C|GetSpline (stale EventBeginPlay _returnvalue))) _新建轨道_0) "World" false)) (.rotation (Spline|GetTransformatDistanceAlongSpline (Variables|/Game/Blueprint/BP_Spline_king1.BP_Spline_king1_C|GetSpline (stale EventBeginPlay _returnvalue)) (Math|Float|Lerp 0.0 (Spline|GetSplineLength (Variables|/Game/Blueprint/BP_Spline_king1.BP_Spline_king1_C|GetSpline (stale EventBeginPlay _returnvalue))) _新建轨道_0) "World" false)) "1.000000,1.000000,1.000000")))
    (:Finished
      (Utilities|FlowControl|Delay 4.0)
      (bind _新建轨道_0_2 (Timeline|时间轴_2 PlayFromStart)
        (:Update
          (Transformation|SetActorTransform (Variables|Default|Getbp_king) (Math|Transform|MakeTransform (.location (Spline|GetTransformatDistanceAlongSpline (Variables|/Game/Blueprint/BP_Spline_king1.BP_Spline_king1_C|GetSpline1 (stale EventBeginPlay _returnvalue)) (Math|Float|Lerp 0.0 (Spline|GetSplineLength (Variables|/Game/Blueprint/BP_Spline_king1.BP_Spline_king1_C|GetSpline1 (stale EventBeginPlay _returnvalue))) _新建轨道_0_2) "World" false)) (.rotation (Spline|GetTransformatDistanceAlongSpline (Variables|/Game/Blueprint/BP_Spline_king1.BP_Spline_king1_C|GetSpline1 (stale EventBeginPlay _returnvalue)) (Math|Float|Lerp 0.0 (Spline|GetSplineLength (Variables|/Game/Blueprint/BP_Spline_king1.BP_Spline_king1_C|GetSpline1 (stale EventBeginPlay _returnvalue))) _新建轨道_0_2) "World" false)) "1.000000,1.000000,1.000000")))
        (:Finished
          (Utilities|FlowControl|Delay 3.0)
          (bind _新建轨道_0_3 (Timeline|时间轴_5 Play)
            (:Update
              (Transformation|SetActorTransform (Variables|Default|Getbp_king) (Math|Transform|MakeTransform (.location (Spline|GetTransformatDistanceAlongSpline _spline2 (Math|Float|Lerp 0.0 (Spline|GetSplineLength _spline2) _新建轨道_0_3) "World" false)) (.rotation (Spline|GetTransformatDistanceAlongSpline _spline2 (Math|Float|Lerp 0.0 (Spline|GetSplineLength _spline2) _新建轨道_0_3) "World" false)) "1.000000,1.000000,1.000000")))
            (:Finished
              (Utilities|FlowControl|Delay 5.0)
              (CallFunction|Looping))))))))

(event EventBeginPlay
  (Utilities|FlowControl|Sequence
    (:then_0
      (bind _returnvalue (Actor|GetActorOfClass "/Game/Blueprint/BP_Spline_king1.BP_Spline_king1_C"))
      (Variables|Default|Setbp_spline_king _returnvalue)
      (bind _returnvalue_2 (Actor|GetActorOfClass "/Game/Blueprint/BP_KING.BP_KING_C"))
      (Variables|Default|Setbp_king _returnvalue_2))
    (:then_1
      ;[0.15 0.15 0.15 0.5] KINGWALK
      (Utilities|FlowControl|Delay 2.0)
      (bind _新建轨道_0 (Timeline|时间轴 Play)
        (:Update
          (Transformation|SetActorTransform (Variables|Default|Getbp_king) (Math|Transform|MakeTransform (.location (Spline|GetTransformatDistanceAlongSpline (Variables|/Game/Blueprint/BP_Spline_king1.BP_Spline_king1_C|GetSpline _returnvalue) (Math|Float|Lerp 0.0 (Spline|GetSplineLength (Variables|/Game/Blueprint/BP_Spline_king1.BP_Spline_king1_C|GetSpline _returnvalue)) _新建轨道_0) "World" false)) (.rotation (Spline|GetTransformatDistanceAlongSpline (Variables|/Game/Blueprint/BP_Spline_king1.BP_Spline_king1_C|GetSpline _returnvalue) (Math|Float|Lerp 0.0 (Spline|GetSplineLength (Variables|/Game/Blueprint/BP_Spline_king1.BP_Spline_king1_C|GetSpline _returnvalue)) _新建轨道_0) "World" false)) "1.000000,1.000000,1.000000")))
        (:Finished
          (Utilities|FlowControl|Delay 4.0)
          (bind _新建轨道_0_2 (Timeline|时间轴_2 PlayFromStart)
            (:Update
              (Transformation|SetActorTransform (Variables|Default|Getbp_king) (Math|Transform|MakeTransform (.location (Spline|GetTransformatDistanceAlongSpline (Variables|/Game/Blueprint/BP_Spline_king1.BP_Spline_king1_C|GetSpline1 _returnvalue) (Math|Float|Lerp 0.0 (Spline|GetSplineLength (Variables|/Game/Blueprint/BP_Spline_king1.BP_Spline_king1_C|GetSpline1 _returnvalue)) _新建轨道_0_2) "World" false)) (.rotation (Spline|GetTransformatDistanceAlongSpline (Variables|/Game/Blueprint/BP_Spline_king1.BP_Spline_king1_C|GetSpline1 _returnvalue) (Math|Float|Lerp 0.0 (Spline|GetSplineLength (Variables|/Game/Blueprint/BP_Spline_king1.BP_Spline_king1_C|GetSpline1 _returnvalue)) _新建轨道_0_2) "World" false)) "1.000000,1.000000,1.000000")))
            (:Finished
              (Utilities|FlowControl|Delay 3.0)
              (bind _新建轨道_0_3 (Timeline|时间轴_5 Play)
                (:Update
                  (Transformation|SetActorTransform (Variables|Default|Getbp_king) (Math|Transform|MakeTransform (.location (Spline|GetTransformatDistanceAlongSpline (Variables|/Game/Blueprint/BP_Spline_king1.BP_Spline_king1_C|GetSpline2 (Variables|Default|Getbp_spline_king)) (Math|Float|Lerp 0.0 (Spline|GetSplineLength (Variables|/Game/Blueprint/BP_Spline_king1.BP_Spline_king1_C|GetSpline2 (Variables|Default|Getbp_spline_king))) _新建轨道_0_3) "World" false)) (.rotation (Spline|GetTransformatDistanceAlongSpline (Variables|/Game/Blueprint/BP_Spline_king1.BP_Spline_king1_C|GetSpline2 (Variables|Default|Getbp_spline_king)) (Math|Float|Lerp 0.0 (Spline|GetSplineLength (Variables|/Game/Blueprint/BP_Spline_king1.BP_Spline_king1_C|GetSpline2 (Variables|Default|Getbp_spline_king))) _新建轨道_0_3) "World" false)) "1.000000,1.000000,1.000000")))
                (:Finished
                  (Utilities|FlowControl|Delay 5.0)
                  (CallFunction|Looping))))))))))

(fn ConstructionScript)