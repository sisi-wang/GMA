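; BP_Painting1 is an interactive painting that can tip over and kills BP_KING on contact with its box.
; Hovering the cursor toggles a highlight, and the BP_Painting event plays a timeline that lerps it from its current location toward a low position while setting pitch flat.
; A box overlap destroys the king, first incrementing the game instance's death count only if the PaintingDie flag is not yet set.
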(event OnComponentBeginOverlap(Box)
  (params (OverlappedComponent :type Primitive%20Component%20Object%20Reference) (OtherActor :type Actor%20Object%20Reference) (OtherComp :type Primitive%20Component%20Object%20Reference) (OtherBodyIndex :type Integer) (bFromSweep :type Boolean) (SweepResult :type Hit%20Result%20Structure%20%28by%20ref%29))
  (bind _asbp_king (Utilities|Casting|CastToBP_KING OtherActor))
  (bind _asbp_ins (Utilities|Casting|CastToBP_INS (Game|GetGameInstance)))
  (if (Variables|/Game/Blueprint/BP_INS.BP_INS_C|Getpainting%20die _asbp_ins)
    _
    (else
      (Variables|/Game/Blueprint/BP_INS.BP_INS_C|Setpainting%20die _asbp_ins true)
      (Variables|/Game/Blueprint/BP_INS.BP_INS_C|Setdie%20number _asbp_ins (+ (Variables|/Game/Blueprint/BP_INS.BP_INS_C|Getdie%20number _asbp_ins) 1))))
  (Actor|DestroyActor _asbp_king))

(event Custom|BP_Painting
  (bind _defaultsceneroot (Variables|Default|GetDefaultSceneRoot))
  (bind _returnvalue (Transformation|GetWorldRotation _defaultsceneroot))
  (bind _returnvalue_2 (Transformation|GetWorldLocation _defaultsceneroot))
  (bind _newtrack_0 (Timeline|Timeline Play)
    (:Update
      (Transformation|SetWorldLocationAndRotation (Variables|Default|GetDefaultSceneRoot) (Math|Vector|Lerp(Vector) (Transformation|GetWorldLocation _defaultsceneroot) (Math|Vector|MakeVector (.x _returnvalue_2) (+ (.y _returnvalue_2) 2e+01) 1e+01) _newtrack_0) (Math|Rotator|MakeRotator (.roll _returnvalue) 9e+01 (.yaw _returnvalue)) false false))))

(event EventBeginPlay)

(event Collision|EventActorBeginOverlap
  (params (OtherActor :type Actor%20Object%20Reference)))

(event EventTick
  (params (DeltaSeconds :type Float%20%28single-precision%29)))

(event MouseInput|EventActorBeginCursorOver
  (Development|SetHiddeninGame (Variables|Default|Getpainting_highlight) false false))

(event MouseInput|EventActorEndCursorOver
  (Development|SetHiddeninGame (Variables|Default|Getpainting_highlight) true false))

(fn ConstructionScript)