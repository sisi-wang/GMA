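; BP_LINE is an actor that traces the navigation path between two BP_point actors as a spline.
; On BeginPlay it caches all BP_point actors and starts a looping timer that drives the update event.
; Each update clears the spline, runs a synchronous navmesh path query between the first two points, and rebuilds the spline from the path points.
; The world-space path points are added in Local spline space.
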(event Custom|update
  (bind _out_actors (Variables|Default|GetOut%20Actors))
  (Spline|ClearSplinePoints (Variables|Default|GetSpline) true)
  (bind _returnvalue (Class|NavigationSystemV1|FindPathtoLocationSynchronously (Transformation|GetActorLocation (Utilities|Array|Get(acopy) _out_actors)) (Transformation|GetActorLocation (Utilities|Array|Get(acopy) _out_actors 1)) self 0))
  (Utilities|IsValid _returnvalue
    (:Is%20Valid
      (if (> (Utilities|Array|Length (Variables|/Script/NavigationSystem.NavigationPath|GetPathPoints _returnvalue)) 0)
        (for _array_element (Variables|/Script/NavigationSystem.NavigationPath|GetPathPoints _returnvalue)
          (Spline|AddSplinePoint (Variables|Default|GetSpline) _array_element "Local" true))
        (Spline|UpdateSpline (Variables|Default|GetSpline))))))

(event EventBeginPlay
  (bind _outactors (Actor|GetAllActorsOfClass "/Game/Blueprint/BP_point.BP_point_C"))
  (Variables|Default|SetOut%20Actors _outactors)
  (Utilities|Time|SetTimerbyEvent (delegate Custom|update) 1.0 true))

(event Collision|EventActorBeginOverlap
  (params (OtherActor :type Actor%20Object%20Reference)))

(event EventTick
  (params (DeltaSeconds :type Float%20%28single-precision%29)))

(fn ConstructionScript)