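; BP_Painting is an interactive painting actor that can move from its place and destroy a BP_KING.
; Cursor hover toggles the PaintingHighlight component's visibility.
; The BP_Painting event plays a timeline that lerps the root from its current location toward a fixed height and negative Y offset, snapping pitch to 90 degrees.
; A BP_KING entering the Box is destroyed after a short delay, independently of the timeline.
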(event OnComponentBeginOverlap(Box)
  (params (OverlappedComponent :type Primitive%20Component%20Object%20Reference) (OtherActor :type Actor%20Object%20Reference) (OtherComp :type Primitive%20Component%20Object%20Reference) (OtherBodyIndex :type Integer) (bFromSweep :type Boolean) (SweepResult :type Hit%20Result%20Structure%20%28by%20ref%29))
  (bind _asbp_king (Utilities|Casting|CastToBP_KING OtherActor))
  (Utilities|FlowControl|Delay 0.5)
  (Actor|DestroyActor _asbp_king))

(event Custom|BP_Painting
  (bind _defaultsceneroot (Variables|Default|GetDefaultSceneRoot))
  (bind _returnvalue (Transformation|GetWorldLocation _defaultsceneroot))
  (bind _returnvalue_2 (Transformation|GetWorldRotation _defaultsceneroot))
  (bind _newtrack_0 (Timeline|Timeline Play)
    (:Update
      (Transformation|SetWorldLocationAndRotation (Variables|Default|GetDefaultSceneRoot) (Math|Vector|Lerp(Vector) (Transformation|GetWorldLocation _defaultsceneroot) (Math|Vector|MakeVector (.x _returnvalue) (+ (.y _returnvalue) -2e+01) 4013.0) _newtrack_0) (Math|Rotator|MakeRotator (.roll _returnvalue_2) 9e+01 (.yaw _returnvalue_2)) false false))))

(event EventBeginPlay)

(event Collision|EventActorBeginOverlap
  (params (OtherActor :type Actor%20Object%20Reference)))

(event EventTick
  (params (DeltaSeconds :type Float%20%28single-precision%29)))

(event MouseInput|EventActorBeginCursorOver
  (Development|SetHiddeninGame (Variables|Default|Getpainting_highlight) false false))

(event MouseInput|EventActorEndCursorOver
  (Development|SetHiddeninGame (Variables|Default|Getpainting_highlight) true false))

(fn ConstructionScript)