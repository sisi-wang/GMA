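; BP_bookbasket is an interactive book basket prop that topples to create a flammable zone and attract the king.
; Its bookbasket event uses a timeline to move and roll the basket to a fixed world position, then spawns BP_FlammableZone there.
; The same event reveals three books, scatters them with delayed timelines, and calls Bookbasket on BP_Gamemode.
; Cursor hover toggles a highlight mesh.
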(event Custom|bookbasket
  (bind _book1 (Variables|Default|Getbook1))
  (bind _book2 (Variables|Default|Getbook2))
  (bind _book3 (Variables|Default|Getbook3))
  (Utilities|FlowControl|Sequence
    (:then_0
      ;[0.15 0.15 0.15 0.5] 书篮时间轴
      (bind _新建轨道_2 (Timeline|Timeline Play)
        (:Update
          (Transformation|SetWorldLocationAndRotation (Variables|Default|Getbookbasket) (Math|Vector|Lerp(Vector) (Transformation|GetWorldLocation (Variables|Default|GetDefaultSceneRoot)) "7271.000000,-3854.000000,4023.000000" _新建轨道_2) (Math|Rotator|MakeRotator (* _新建轨道_2 1.8e+02) 0.0 0.0) false false))
        (:Finished
          ;[0.15 0.15 0.15 0.5] 生成易燃区
          (Game|SpawnActorfromClass "/Game/Blueprint/BP_FlammableZone.BP_FlammableZone_C" (Math|Transform|MakeTransform (Transformation|GetWorldLocation (Variables|Default|Getbookbasket)) "0, 0, 0" "2.500000,2.500000,2.500000") "Undefined" "MultiplyWithRoot" 0 0))))
    (:then_1
      ;[0.15 0.15 0.15 0.5] 书蓝中的书时间轴
      (Development|SetHiddeninGame (Variables|Default|Getbook2) false false)
      (Development|SetHiddeninGame (Variables|Default|Getbook1) false false)
      (Development|SetHiddeninGame (Variables|Default|Getbook3) false false)
      (Utilities|FlowControl|Sequence
        (:then_0
          (Utilities|FlowControl|Delay 0.2)
          (bind _新建轨道_2_2 (Timeline|Timeline_0 Play)
            (:Update
              (Transformation|SetWorldLocationAndRotation _book1 (Math|Vector|Lerp(Vector) (Transformation|GetWorldLocation _book1) "7215.000000,-3845.000000,4005.000000" _新建轨道_2_2) (Math|Rotator|MakeRotator 156.0 9e+01 176.0) false false))))
        (:then_1
          (Utilities|FlowControl|Delay 0.2)
          (bind _新建轨道_2_3 (Timeline|Timeline_1 Play)
            (:Update
              (Transformation|SetWorldLocationAndRotation _book2 (Math|Vector|Lerp(Vector) (Transformation|GetWorldLocation _book2) "7237.000000,-3806.000000,4003.000000" _新建轨道_2_3) (Math|Rotator|MakeRotator 0.0 0.0 0.0) false false))))
        (:then_2
          (Utilities|FlowControl|Delay 0.2)
          (bind _新建轨道_2_4 (Timeline|Timeline_2 Play)
            (:Update
              (Transformation|SetWorldLocationAndRotation _book3 (Math|Vector|Lerp(Vector) (Transformation|GetWorldLocation _book3) "7357.000000,-3823.000000,4003.000000" _新建轨道_2_4) (Math|Rotator|MakeRotator 0.0 0.0 0.0) false false))))))
    (:then_2
      ;[0.15 0.15 0.15 0.5] 书蓝掉落吸引king
      (bind _asbp_gamemode (Utilities|Casting|CastToBP_Gamemode (Game|GetGameMode)))
      (Default|Bookbasket _asbp_gamemode))))

(event EventBeginPlay)

(event Collision|EventActorBeginOverlap
  (params (OtherActor :type Actor%20Object%20Reference)))

(event EventTick
  (params (DeltaSeconds :type Float%20%28single-precision%29)))

(event MouseInput|EventActorBeginCursorOver
  (Development|SetHiddeninGame (Variables|Default|GetBookbasket_highlight) false false))

(event MouseInput|EventActorEndCursorOver
  (Development|SetHiddeninGame (Variables|Default|GetBookbasket_highlight) true false))

(fn ConstructionScript)