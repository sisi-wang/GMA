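; BP_FlammableZone is a trigger zone that catches fire when a candlestick tagged Flammable overlaps its box.
; The box tracks whether BP_KING is inside and identifies candlesticks by display name.
; Ignition spawns two fire emitters, then either destroys the King after a short delay if inside, or calls FireBookbasket on BP_Gamemode, commented as stopping walking at the sight of fire.
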(event OnComponentEndOverlap(Box)
  (params (OverlappedComponent :type Primitive%20Component%20Object%20Reference) (OtherActor :type Actor%20Object%20Reference) (OtherComp :type Primitive%20Component%20Object%20Reference) (OtherBodyIndex :type Integer))
  (Utilities|Casting|CastToBP_KING OtherActor)
  (Variables|Default|SetIn%20Box false))

(event OnComponentBeginOverlap(Box)
  (params (OverlappedComponent :type Primitive%20Component%20Object%20Reference) (OtherActor :type Actor%20Object%20Reference) (OtherComp :type Primitive%20Component%20Object%20Reference) (OtherBodyIndex :type Integer) (bFromSweep :type Boolean) (SweepResult :type Hit%20Result%20Structure%20%28by%20ref%29))
  (switch name (Utilities|String|StringToName (Utilities|GetDisplayName OtherActor))
    (:BP_Candlestick
      (if (Utilities|Array|ContainsItem (Variables|/Script/Engine.Actor|GetTags OtherActor) "Flammable") :!label _label
        (CallFunction|FireFX)
        (if (Variables|Default|GetIn%20Box)
          (CallFunction|FireDestroyactor)
          (else
            (CallFunction|FireStopwalk)))))
    (:BP_KING
      (Variables|Default|SetIn%20Box true))
    (:BP_Candlestick1
      (goto _label))))

(event Custom|Fire_FX
  (bind _box (Variables|Default|GetBox))
  (bind _returnvalue (Transformation|GetWorldLocation _box))
  (bind _returnvalue_2 (- (.z _returnvalue) 8e+01))
  ;[0.15 0.15 0.15 0.5] 火粒子
  (Effects|SpawnEmitteratLocation "/Game/PolygonFantasyKingdom/FX/FX_Fire.FX_Fire" (Math|Vector|MakeVector (+ (.x _returnvalue) 1e+02) (- (.y _returnvalue) 5e+01) _returnvalue_2))
  (Effects|SpawnEmitteratLocation "/Game/PolygonFantasyKingdom/FX/FX_Fire.FX_Fire" (Math|Vector|MakeVector (- (.x _returnvalue) 5e+01) (.y _returnvalue) _returnvalue_2)))

(event Custom|Fire_stopwalk
  ;[0.15 0.15 0.15 0.5] 看见火停止行走
  (bind _asbp_gamemode (Utilities|Casting|CastToBP_Gamemode (Game|GetGameMode)))
  (Default|FireBookbasket _asbp_gamemode))

(event Custom|Fire_destroyactor
  ;[0.15 0.15 0.15 0.5] 销毁king
  (Utilities|FlowControl|Delay 0.8)
  (bind _returnvalue (Actor|GetActorOfClass "/Game/Blueprint/BP_KING.BP_KING_C"))
  (Actor|DestroyActor _returnvalue))

(event EventBeginPlay)

(event Collision|EventActorBeginOverlap
  (params (OtherActor :type Actor%20Object%20Reference))
  ;[0.15 0.15 0.15 0.5] 火粒子
)

(fn ConstructionScript)