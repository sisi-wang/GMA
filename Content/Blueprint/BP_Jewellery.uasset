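; BP_Jewellery is a jewellery actor that highlights under the cursor and can be moved to a fixed world location.
; Cursor over and out events show and hide the JewelleryHighlight component.
; The BP_jewellery event plays a timeline that lerps from the actor's current location, re-read each update, toward that hard-coded point.
; Each timeline update also calls Jewellery on BP_Gamemode, so that call repeats throughout playback.
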(event Custom|BP_jewellery
  (bind _returnvalue (Transformation|GetActorLocation))
  (bind _新建轨道_2 (Timeline|时间轴 Play)
    (:Update
      (Transformation|SetActorLocation (Math|Vector|Lerp(Vector) (Math|Vector|MakeVector (.x _returnvalue) (.y _returnvalue) (.z _returnvalue)) (Math|Vector|MakeVector 7833.0 -2969.0 4001.0) _新建轨道_2) false false)
      (bind _asbp_gamemode (Utilities|Casting|CastToBP_Gamemode (Game|GetGameMode)))
      (Default|Jewellery _asbp_gamemode))))

(event EventBeginPlay)

(event Collision|EventActorBeginOverlap
  (params (OtherActor :type Actor%20Object%20Reference)))

(event EventTick
  (params (DeltaSeconds :type Float%20%28single-precision%29)))

(event MouseInput|EventActorBeginCursorOver
  (Development|SetHiddeninGame (Variables|Default|GetJewellery_highlight) false false))

(event MouseInput|EventActorEndCursorOver
  (Development|SetHiddeninGame (Variables|Default|GetJewellery_highlight) true false))

(fn ConstructionScript)