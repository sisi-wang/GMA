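; BP_WINE is an interactive wine bottle that tips over and leaves a flammable area behind.
; The BP_Wine event plays a timeline that moves the bottle mesh from the actor root to a hardcoded world position while rolling it onto its side.
; When the timeline finishes, it spawns an enlarged BP_FlammableZone at the bottle's location.
; Cursor-over events show and hide the WINEHIGHLIGHT component as hover feedback.
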(event Custom|BP_Wine
  ;[0.15 0.15 0.15 0.5] 书篮时间轴
  (bind _新建轨道_2 (Timeline|时间轴 Play)
    (:Update
      (Transformation|SetWorldLocationAndRotation (Variables|Default|GetSM_Item_Bottle_04) (Math|Vector|Lerp(Vector) (Transformation|GetWorldLocation (Variables|Default|GetDefaultSceneRoot)) "6786.000000,-2637.000000,4012.000000" _新建轨道_2) (Math|Rotator|MakeRotator (* _新建轨道_2 9e+01) 0.0 0.0) false false))
    (:Finished
      ;[0.15 0.15 0.15 0.5] 生成易燃区
      (Game|SpawnActorfromClass "/Game/Blueprint/BP_FlammableZone.BP_FlammableZone_C" (Math|Transform|MakeTransform (Transformation|GetWorldLocation (Variables|Default|GetSM_Item_Bottle_04)) "0, 0, 0" "3.000000,3.000000,3.000000") "Undefined" "MultiplyWithRoot" 0 0))))

(event EventBeginPlay)

(event Collision|EventActorBeginOverlap
  (params (OtherActor :type Actor%20Object%20Reference)))

(event EventTick
  (params (DeltaSeconds :type Float%20%28single-precision%29)))

(event MouseInput|EventActorBeginCursorOver
  (Development|SetHiddeninGame (Variables|Default|GetWINE%29HIGHLIGHT) false false))

(event MouseInput|EventActorEndCursorOver
  (Development|SetHiddeninGame (Variables|Default|GetWINE%29HIGHLIGHT) true false))

(fn ConstructionScript)