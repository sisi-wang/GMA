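; BP_Candlestick is a candlestick actor that shows a highlight mesh under the cursor and can be knocked over.
; Its Candlestick event plays a timeline that rotates the mesh in place into a tipped pose, with a metal crash sound shortly after it starts.
; When the timeline finishes, it clears the actor's tags and, after a short delay, destroys the point light.
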(event Custom|Candlestick
  (bind _candlestick (Variables|Default|GetCandlestick))
  (Utilities|FlowControl|Sequence
    (:then_0
      (Utilities|FlowControl|Delay 0.1)
      (Audio|SpawnSoundatLocation "/Game/Music/ES_Metal__Impact__Hit__Garbage_Junkyard__Crash_-_Epidemic_Sound_-_32421-35530.ES_Metal__Impact__Hit__Garbage_Junkyard__Crash_-_Epidemic_Sound_-_32421-35530" (Transformation|GetActorLocation) "0, 0, 0" 1.0 1.0 0.0 0 0))
    (:then_1
      (bind _新建轨道_2 (Timeline|时间轴 Play)
        (:Update
          (Transformation|SetWorldLocationAndRotation _candlestick (Transformation|GetWorldLocation _candlestick) (Math|Rotator|MakeRotator (* _新建轨道_2 -87.0) 0.0 (* _新建轨道_2 -45.0)) false false))
        (:Finished
          (Utilities|Array|Clear (Variables|Actor|GetTags))
          (Utilities|FlowControl|Delay 2.0)
          (Components|DestroyComponent (Variables|Default|GetPointLight)))))))

(event EventBeginPlay)

(event Collision|EventActorBeginOverlap
  (params (OtherActor :type Actor%20Object%20Reference)))

(event EventTick
  (params (DeltaSeconds :type Float%20%28single-precision%29)))

(event MouseInput|EventActorBeginCursorOver
  (Development|SetHiddeninGame (Variables|Default|GetCandlestick_highlight) false false))

(event MouseInput|EventActorEndCursorOver
  (Development|SetHiddeninGame (Variables|Default|GetCandlestick_highlight) true false))

(fn ConstructionScript)