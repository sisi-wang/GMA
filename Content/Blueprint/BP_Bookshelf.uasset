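; BP_Bookshelf is a bookshelf hazard that can topple and kill BP_KING, showing a highlight while the cursor hovers over it.
; Its Bookshelf event plays a timeline that rolls the root over, then removes the Box trigger shortly after it finishes.
; When BP_KING overlaps the Box, it is destroyed after a short delay, and BP_INS counts this death type only once through the BookshelfDie flag and DieNumber.
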(event OnComponentBeginOverlap(Box)
  (params (OverlappedComponent :type Primitive%20Component%20Object%20Reference) (OtherActor :type Actor%20Object%20Reference) (OtherComp :type Primitive%20Component%20Object%20Reference) (OtherBodyIndex :type Integer) (bFromSweep :type Boolean) (SweepResult :type Hit%20Result%20Structure%20%28by%20ref%29))
  (bind _asbp_king (Utilities|Casting|CastToBP_KING OtherActor))
  (Utilities|FlowControl|Delay 0.2)
  (bind _asbp_ins (Utilities|Casting|CastToBP_INS (Game|GetGameInstance)))
  (if (Variables|/Game/Blueprint/BP_INS.BP_INS_C|Getbookshelf%20die _asbp_ins)
    _
    (else
      (Variables|/Game/Blueprint/BP_INS.BP_INS_C|Setbookshelf%20die _asbp_ins true)
      (Variables|/Game/Blueprint/BP_INS.BP_INS_C|Setdie%20number _asbp_ins (+ (Variables|/Game/Blueprint/BP_INS.BP_INS_C|Getdie%20number _asbp_ins) 1))))
  (Actor|DestroyActor _asbp_king))

(event Custom|Bookshelf
  (bind _defaultsceneroot (Variables|Default|GetDefaultSceneRoot))
  (bind _新建轨道_2 (Timeline|时间轴 Play)
    (:Update
      (Transformation|SetWorldLocationAndRotation _defaultsceneroot (Transformation|GetWorldLocation _defaultsceneroot) (Math|Rotator|MakeRotator (* _新建轨道_2 9e+01) 0.0 0.0) false false))
    (:Finished
      (Utilities|FlowControl|Delay 0.2)
      (Components|DestroyComponent (Variables|Default|GetBox)))))

(event EventBeginPlay)

(event Collision|EventActorBeginOverlap
  (params (OtherActor :type Actor%20Object%20Reference)))

(event EventTick
  (params (DeltaSeconds :type Float%20%28single-precision%29)))

(event MouseInput|EventActorBeginCursorOver
  (Development|SetHiddeninGame (Variables|Default|GetBookshelf_highlight) false false))

(event MouseInput|EventActorEndCursorOver
  (Development|SetHiddeninGame (Variables|Default|GetBookshelf_highlight) true false))

(fn ConstructionScript)