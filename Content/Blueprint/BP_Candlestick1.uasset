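; BP_Candlestick1 is an interactable candlestick actor with a cursor hover highlight and a one-way rotation animation.
; Cursor begin and end events show and hide the CandlestickHighlight component.
; The custom Candlestick event, with no caller in this file, plays a timeline that scales the Candlestick component's world roll and yaw by -90 degrees at its current location.
; When the timeline finishes, the actor's Tags are cleared.
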(event Custom|Candlestick
  (bind _candlestick (Variables|Default|GetCandlestick))
  (bind _新建轨道_2 (Timeline|时间轴 Play)
    (:Update
      (Transformation|SetWorldLocationAndRotation _candlestick (Transformation|GetWorldLocation _candlestick) (Math|Rotator|MakeRotator (* _新建轨道_2 -9e+01) 0.0 (* _新建轨道_2 -9e+01)) false false))
    (:Finished
      (Utilities|Array|Clear (Variables|Actor|GetTags)))))

(event EventBeginPlay)

(event Collision|EventActorBeginOverlap
  (params (OtherActor :type Actor%20Object%20Reference)))

(event EventTick
  (params (DeltaSeconds :type Float%20%28single-precision%29)))

(event MouseInput|EventActorBeginCursorOver
  (Development|SetHiddeninGame (Variables|Default|GetCandlestick_highlight) false false))

(event MouseInput|EventActorEndCursorOver
  (Development|SetHiddeninGame (Variables|Default|GetCandlestick_highlight) true false))

(fn ConstructionScript)